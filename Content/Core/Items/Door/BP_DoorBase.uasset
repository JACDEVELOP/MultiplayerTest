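; BP_DoorBase is a base door that toggles open and closed when interacted with.
; On BeginPlay it binds to a door interaction delegate, whose event alternates a timeline between play and reverse through a FlipFlop.
; Timeline alpha drives DoorTransform, which lerps the static mesh's relative transform from a hard-coded closed pose toward SlideLocation and RotationAmount, supporting sliding or rotating motion.
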(event Custom|DoorInteraction
  (Utilities|FlowControl|FlipFlop
    (:A
      (bind _alpha (Timeline|TL_Door Play)
        (:Update
          (CallFunction|DoorTransform _alpha))))
    (:B
      (Timeline|TL_Door Reverse))))

(event EventBeginPlay
  (EventDispatchers|BindEventtoDoorInteractionDelegate (delegate Custom|DoorInteraction)))

(fn ConstructionScript)

(fn DoorTransform
  (params (Alpha :type Float%20%28single-precision%29))
  (Transformation|SetRelativeTransform (Variables|Default|GetStaticMeshComponent) (Math|Transform|Lerp(Transform) (Math|Transform|MakeTransform "0.000000,46.000000,-101.000000") (Math|Transform|MakeTransform (Variables|Default|GetSlideLocation) (Variables|Default|GetRotationAmount) "1.000000,1.000000,1.000000") Alpha "EulerInterp") false false))